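; Beat Cube is an actor that shuttles back and forth along a movement vector each time its beat function is triggered.
; Each beat stores the current location, flips the sign of MoveVec and replays a timeline that offsets the cube from that location by the vector scaled by timeline progress.
; BeginPlay also caches the starting location and flips the vector once.
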(event EventBeginPlay
  ;[1 1 1] 初期化
  (Variables|Default|SetCurrentCoord (Transformation|GetWorldLocation (Variables|Transformation|GetRootComponent)))
  (Variables|Default|SetMoveVec (* (Variables|Default|GetMoveVec) -1.0)))

(event EventBeatFunction
  ;[1 1 1] Beat Event
  (Variables|Default|SetCurrentCoord (Transformation|GetWorldLocation (Variables|Transformation|GetRootComponent)))
  (Variables|Default|SetMoveVec (* (Variables|Default|GetMoveVec) -1.0))
  (bind _progress (Timeline|BeatLine PlayFromStart)
    (:Update
      (Transformation|SetWorldLocation (Variables|Transformation|GetRootComponent) (+ (* (Variables|Default|GetMoveVec) _progress) (Variables|Default|GetCurrentCoord)) false false))))

(fn ConstructionScript)